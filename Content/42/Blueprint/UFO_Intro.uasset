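; UFO_Intro is an intro actor that pulls the VR player pawn toward a target point.
; On BeginPlay it caches the level's VRPawn as the player.
; StartUpPlayer stores a target, waits briefly, records the player's location and enables movement.
; Each Tick then moves the pawn a small fixed fraction of the remaining distance, giving a frame-rate-dependent ease-out while keeping its rotation.
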(event Custom|StartUpPlayer
  (params (TargetLocation :type Vector))
  (Variables|Default|SetTargetLocation TargetLocation)
  (Utilities|FlowControl|Delay 0.2)
  (Variables|Default|Setlocation (Transformation|GetActorLocation (Variables|Default|GetPlayer)))
  (Variables|Default|SetSubstract true))

(event EventBeginPlay
  (bind _returnvalue (Actor|GetActorOfClass "/Game/VRTemplate/Blueprints/VRPawn.VRPawn_C"))
  (bind _asvrpawn (Utilities|Casting|CastToVRPawn _returnvalue))
  (Variables|Default|SetPlayer _asvrpawn))

(event Collision|EventActorBeginOverlap
  (params (OtherActor :type Actor%20Object%20Reference)))

(event EventTick
  (params (DeltaSeconds :type Float%20%28single-precision%29))
  (bind _player (Variables|Default|GetPlayer))
  (if (Variables|Default|GetSubstract)
    (Transformation|SetActorTransform _player (Math|Transform|MakeTransform (Variables|Default|Getlocation) (Transformation|GetActorRotation _player)))
    (Variables|Default|Setlocation (+ (Variables|Default|Getlocation) (* (- (Variables|Default|GetTargetLocation) (Variables|Default|Getlocation)) (Math|Conversions|ToVector(Float) 0.002))))))

(fn ConstructionScript)